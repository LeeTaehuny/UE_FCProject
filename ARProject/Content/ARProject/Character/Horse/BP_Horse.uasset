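; BP_Horse is a rideable horse that the player possesses to ride, with look, forward-axis movement and adjustable spring-arm camera length and offset.
; Overlapping RidePosition binds HorseRide to BP_Player, and leaving unbinds it.
; HorseRide caches the player, possesses the horse and shows its own Player component as a stand-in rider.
; IA_Ride dismounts by moving the cached player to UnRidePosition, repossessing them and hiding the stand-in.
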(event `EnhancedInput|/Game/ARProject/Character/Controller/InputAction/IA_Look`
  (params (ActionValue :type "Vector2D Structure") (ElapsedSeconds :type "Float (double-precision)") (TriggeredSeconds :type "Float (double-precision)") (InputAction :type "InputAction Object Reference" :default "/Game/ARProject/Character/Controller/InputAction/IA_Look.IA_Look"))
  ;[1 1 1] Look
  (:`Triggered`
    (`self.AddControllerYawInput` ActionValue_X)
    (`self.AddControllerPitchInput` ActionValue_Y)))

(event `EnhancedInput|/Game/ARProject/Character/Controller/InputAction/IA_CameraLength`
  (params (ActionValue :type "Float (double-precision)") (ElapsedSeconds :type "Float (double-precision)") (TriggeredSeconds :type "Float (double-precision)") (InputAction :type "InputAction Object Reference" :default "/Game/ARProject/Character/Controller/InputAction/IA_CameraLength.IA_CameraLength"))
  ;[1 1 1] Camera Length
  (:`Triggered`
    (set `SpringArmComponent.TargetArmLength` (`KismetMathLibrary.FClamp` (+ (`SpringArmComponent.TargetArmLength` (`self.SpringArm`)) (* ActionValue 50.0)) 300.0 800.0) (`self.SpringArm`))))

(event `EnhancedInput|/Game/ARProject/Character/Controller/InputAction/IA_CameraPosition`
  (params (ActionValue :type "Vector2D Structure") (ElapsedSeconds :type "Float (double-precision)") (TriggeredSeconds :type "Float (double-precision)") (InputAction :type "InputAction Object Reference" :default "/Game/ARProject/Character/Controller/InputAction/IA_CameraPosition.IA_CameraPosition"))
  ;[1 1 1] Camera Position
  (:`Triggered`
    (`SceneComponent.K2_AddLocalOffset` (`self.SpringArm`) (`KismetMathLibrary.MakeVector` 0.0 ActionValue_X ActionValue_Y) false false)))

(event `self.RidePosition.OnComponentBeginOverlap`
  (params (OverlappedComponent :type "PrimitiveComponent Object Reference") (OtherActor :type "Actor Object Reference") (OtherComp :type "PrimitiveComponent Object Reference") (OtherBodyIndex :type Integer) (bFromSweep :type Boolean) (SweepResult :type "HitResult Structure (by ref)"))
  (bind _asbp_player (cast `/Game/ARProject/Character/Player/Blueprint/BP_Player` OtherActor))
  (add `/Game/ARProject/Character/Player/Blueprint/BP_Player.HorseRide` _asbp_player (delegate `HorseRide`)))

(event `EnhancedInput|/Game/ARProject/Character/Controller/InputAction/IA_Move`
  (params (ActionValue :type "Vector2D Structure") (ElapsedSeconds :type "Float (double-precision)") (TriggeredSeconds :type "Float (double-precision)") (InputAction :type "InputAction Object Reference" :default "/Game/ARProject/Character/Controller/InputAction/IA_Move.IA_Move"))
  ;[1 1 1] Move
  (:`Triggered`
    (bind _output_get (set `self.ForwardInput` ActionValue_Y))
    (`self.AddMovementInput` (`self.GetActorForwardVector`) _output_get))
  (:`Completed`
    (set `self.ForwardInput` 0.0)))

(event `self.RidePosition.OnComponentEndOverlap`
  (params (OverlappedComponent :type "PrimitiveComponent Object Reference") (OtherActor :type "Actor Object Reference") (OtherComp :type "PrimitiveComponent Object Reference") (OtherBodyIndex :type Integer))
  (bind _asbp_player (cast `/Game/ARProject/Character/Player/Blueprint/BP_Player` OtherActor))
  (remove `/Game/ARProject/Character/Player/Blueprint/BP_Player.HorseRide` _asbp_player (delegate `HorseRide`)))

(event `HorseRide`
  (bind _asbp_player (cast `/Game/ARProject/Character/Player/Blueprint/BP_Player` (`GameplayStatics.GetPlayerCharacter` 0)))
  (set `self.As BP Player` _asbp_player)
  (`Controller.Possess` (`GameplayStatics.GetPlayerController` 0) self)
  (`SceneComponent.SetVisibility` (`self.Player`) true false))

(event `EnhancedInput|/Game/ARProject/Character/Controller/InputAction/IA_Ride`
  (params (ActionValue :type Boolean) (ElapsedSeconds :type "Float (double-precision)") (TriggeredSeconds :type "Float (double-precision)") (InputAction :type "InputAction Object Reference" :default "/Game/ARProject/Character/Controller/InputAction/IA_Ride.IA_Ride"))
  (bind _unrideposition (`self.UnRidePosition`))
  (:`Started`
    (`/Engine/EditorBlueprintResources/StandardMacros.IsValid` (`self.As BP Player`)
      (:`Is Valid`
        (`self.K2_SetActorTransform` (`self.As BP Player`) (`KismetMathLibrary.MakeTransform` (`SceneComponent.K2_GetComponentLocation` _unrideposition) (`SceneComponent.K2_GetComponentRotation` _unrideposition)) false false)
        (`Controller.Possess` (`GameplayStatics.GetPlayerController` 0) (`self.As BP Player`))
        (`SceneComponent.SetVisibility` (`self.Player`) false false)))))

(fn `UserConstructionScript`)