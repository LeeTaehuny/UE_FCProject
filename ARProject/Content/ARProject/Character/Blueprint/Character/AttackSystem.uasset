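; AttackSystem is a component that handles weapon hit detection and damage for its owning BP_BaseCharacter.
; StartWeaponTrace runs a fast looping timer that sphere-traces between the character's weapon top and bottom, with debug drawing, until StopWeaponTrace clears it.
; A hit applies fixed damage through a DoOnce that resets after a short delay, limiting repeat hits across all targets.
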(event `self.ReceiveBeginPlay`
  (bind _asbp_base_character (cast `/Game/ARProject/Character/Blueprint/Character/BP_BaseCharacter` (`self.GetOwner`)))
  (set `self.As BP Base Character` _asbp_base_character))

(event `StartWeaponTrace`
  (bind _returnvalue (`KismetSystemLibrary.K2_SetTimerDelegate` (delegate `WeaponTraceLoop`) 0.01 true))
  (set `self.TraceLoop` _returnvalue))

(event `WeaponTraceLoop`
  (bind _as_bp_base_character (`self.As BP Base Character`))
  (bind _position (`/Game/ARProject/Character/Blueprint/Character/BP_BaseCharacter.GetWeaponTop` _as_bp_base_character))
  (bind _position_2 (`/Game/ARProject/Character/Blueprint/Character/BP_BaseCharacter.GetWeaponBottom` _as_bp_base_character))
  (bind (_outhit _returnvalue) (`KismetSystemLibrary.SphereTraceSingle` :`Start` _position :`End` _position_2 :`Radius` 12.0 :`TraceChannel` "TraceTypeQuery3" :`DrawDebugType` "ForDuration"))
  (if _returnvalue
    (`/Engine/EditorBlueprintResources/StandardMacros.DoOnce` false :!label _label
      (:`Completed`
        (`GameplayStatics.ApplyDamage` (`.HitActor` (`GameplayStatics.BreakHitResult` _outhit)) 100.0)
        (`KismetSystemLibrary.Delay` 0.5)
        (goto _label :!via `Reset`)))))

(event `StopWeaponTrace`
  (`KismetSystemLibrary.K2_ClearAndInvalidateTimerHandle` (`self.TraceLoop`)))